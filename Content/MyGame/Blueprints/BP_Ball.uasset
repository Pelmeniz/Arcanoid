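; BP_Ball is a bouncing ball that moves in the XY plane and speeds up with each hit.
; Tick moves the Sphere component by Direction, Speed and delta time using a swept world offset rather than physics simulation.
; On a blocking hit it reflects Direction about the surface normal, plays a touch sound and adds AddedSpeed to Speed up to a fixed cap.
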(event `self.ReceiveTick`
  (params (DeltaSeconds :type "Float (single-precision)"))
  (bind (_returnvalue_x _returnvalue_y) (`KismetMathLibrary.BreakVector` (* (* DeltaSeconds (`self.Speed`)) (`self.Direction`))))
  ;[1 0.2757 0.2956] Движение мяча с увеличением скорости
  (bind _sweephitresult (`SceneComponent.K2_AddWorldOffset` (`self.Sphere`) (`KismetMathLibrary.MakeVector` _returnvalue_x _returnvalue_y) true false))
  (bind (_bblockinghit _binitialoverlap _time _distance _location _impactpoint _normal) (`GameplayStatics.BreakHitResult` _sweephitresult))
  (if _bblockinghit
    (set `self.Direction` (`KismetMathLibrary.GetReflectionVector` (`self.Direction`) _normal))
    (`GameplayStatics.PlaySoundAtLocation` "/Game/MyGame/Sounds/A_BallToch_Cue.A_BallToch_Cue" (`self.K2_GetActorLocation`) (struct) 1.0 1.0 0.0 null null null null)
    (set `self.Speed` (`KismetMathLibrary.FMin` (+ (`self.Speed`) (`self.AddedSpeed`)) 2000.0))))

(fn `UserConstructionScript`)