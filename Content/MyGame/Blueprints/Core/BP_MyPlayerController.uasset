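; Player controller for a paddle-and-ball cube-breaking game that runs the HUD, input and end-of-match flow.
; It creates the HUD, forwards axis and action input to the possessed BP_MyPawn for sweep movement and ball spawning, and opens the menu map on Exit.
; The cube generator's all-cubes-died event triggers a win and the pawn's game-end event a loss, both sharing one result screen path with sound and UI-only input.
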(event `self.ReceiveBeginPlay`
  (`|ExecutionSequence`
    (:`then_0`
      ;[1 0.4631 0.6249] Автопереключение в игру
      (`WidgetBlueprintLibrary.SetInputMode_GameOnly` self)
      (bind _returnvalue (`|CreateWidget` "/Game/MyGame/UI/WBP_HUD.WBP_HUD_C" self))
      (`UserWidget.AddToViewport` _returnvalue 0)
      (set `self.HUD` _returnvalue))
    (:`then_1`
      ;[1 0.5185 0.4886] Screen при победе или поражении
      (bind _returnvalue_2 (`GameplayStatics.GetActorOfClass` "/Game/MyGame/Blueprints/BP_CubesGenerator.BP_CubesGenerator_C"))
      (add `/Game/MyGame/Blueprints/BP_CubesGenerator.AllCubesDied` _returnvalue_2 (delegate `GameFinished`)))))

(event `GameFinished`
  ;[1 0.5185 0.4886] Screen при победе или поражении
  (set `self.bIsWinner` true)
  (`GameplayStatics.PlaySound2D` "/Game/MyGame/Sounds/A_Win_Cue.A_Win_Cue" 1.0 1.0 0.0 null null)
  (`Widget.SetVisibility` (`self.HUD`) "Collapsed" :!label _label)
  (bind _returnvalue (`|CreateWidget` "/Game/MyGame/UI/WBP_WinScreen.WBP_WinScreen_C" self))
  (`/Game/MyGame/UI/WBP_WinScreen.UpdateWinner` _returnvalue (`self.bIsWinner`))
  (`UserWidget.AddToViewport` _returnvalue 0)
  (`WidgetBlueprintLibrary.SetInputMode_UIOnlyEx` self _returnvalue "LockOnCapture")
  (set `self.bShowMouseCursor` true))

(event `PlayerDDie`
  ;[1 0.5185 0.4886] Screen при победе или поражении
  (set `self.bIsWinner` false)
  (`GameplayStatics.PlaySound2D` "/Game/MyGame/Sounds/A_Lose_Cue.A_Lose_Cue" 1.0 1.0 0.0 null null)
  (goto _label))

(event `self.ReceivePossess`
  (params (PossessedPawn :type "Pawn Object Reference"))
  ;[1 0.8338 0.5895] Каретка
  (bind _asbp_my_pawn (cast `/Game/MyGame/Blueprints/Core/BP_MyPawn` PossessedPawn))
  (bind _output_get (set `self.MyPawn` _asbp_my_pawn))
  ;[1 0.5185 0.4886] Screen при победе или поражении
  (add `/Game/MyGame/Blueprints/Core/BP_MyPawn.GameEnd` _output_get (delegate `PlayerDDie`)))

(event `InputAxis|Left_Right`
  (params (AxisValue :type "Float (single-precision)"))
  ;[0.2282 0.7251 1] Управление кареткой в мире
  (`self.K2_AddActorWorldOffset` (`self.MyPawn`) (`KismetMathLibrary.MakeVector` 0.0 (* AxisValue (`GameplayStatics.GetWorldDeltaSeconds`) (`self.Speed`))) true false))

(event `InputAction|SpawnBall`
  (params (Key :type "Key Structure"))
  ;[0.2768 1 0.4154] Spawn Ball
  (:`Pressed`
    (`/Game/MyGame/Blueprints/Core/BP_MyPawn.SpawnBall` (`self.MyPawn`))))

(event `InputAction|Exit`
  (params (Key :type "Key Structure"))
  (:`Pressed`
    (`GameplayStatics.OpenLevelBySoftObjectPtr` "/Game/MyGame/Levels/MenuMap.MenuMap")))

(fn `UserConstructionScript`)