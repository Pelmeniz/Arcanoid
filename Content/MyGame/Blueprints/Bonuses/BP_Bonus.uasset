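; BP_Bonus is a moving bonus actor that carries one of three randomly chosen bonus types.
; The Construction Script rolls BonusType at random and writes its enum name to a TextRender label.
; Tick moves the Cylinder component with a swept world offset from Speed, Direction and delta time, using only the X component.
; The graph contains no pickup or effect logic.
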(event `self.ReceiveTick`
  (params (DeltaSeconds :type "Float (single-precision)"))
  (bind _returnvalue_x (`KismetMathLibrary.BreakVector` (* (* DeltaSeconds (`self.Speed`)) (`self.Direction`))))
  ;[1 0.2757 0.2956] Движение мяча с увеличением скорости
  (`SceneComponent.K2_AddWorldOffset` (`self.Cylinder`) (`KismetMathLibrary.MakeVector` _returnvalue_x) true false))

(fn `UserConstructionScript`
  (set `self.BonusType` (select `int` (`KismetMathLibrary.RandomIntegerInRange` 0 2) :`0` "NewEnumerator0" :`1` "NewEnumerator1" :`2` "NewEnumerator2" :!type "/Game/MyGame/Blueprints/Bonuses/E_BonusType Enum"))
  (`TextRenderComponent.K2_SetText` (`self.TextRender`) (`KismetTextLibrary.Conv_StringToText` (`|GetEnumeratorNameAsString` (`self.BonusType`)))))