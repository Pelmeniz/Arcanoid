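; BP_Cube_Child is a cube variant, hit by a ball, that can drop a bonus pickup when destroyed.
; On BeginPlay it binds a spawn handler to its destroyed event only if the cube's first material is BasicAsset01.
; The handler always spawns BP_Bonus at the cube's location with a fixed rotation.
; Hit handling and construction defer to the parent Blueprint.
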(event `self.ReceiveBeginPlay`
  (if (== (`PrimitiveComponent.GetMaterial` (`self.Cube`) 0) "/Engine/MapTemplates/Materials/BasicAsset01.BasicAsset01")
    (add `self.OnDestroyed` (delegate `SpawnBonus`))))

(event `SpawnBonus` :!signature `self.OnDestroyed`
  (params (DestroyedActor :type "Actor Object Reference"))
  (`|SpawnActorFromClass` "/Game/MyGame/Blueprints/Bonuses/BP_Bonus.BP_Bonus_C" (`KismetMathLibrary.MakeTransform` (`self.K2_GetActorLocation`) (struct :`Pitch` 90.0)) "AlwaysSpawn" "MultiplyWithRoot" null null))

(event `self.BallIsHit`
  (`parent.BallIsHit`))

(fn `UserConstructionScript`
  (`parent.UserConstructionScript`))