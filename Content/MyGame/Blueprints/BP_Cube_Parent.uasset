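; BP_Cube_Parent is a breakable cube that is damaged by BP_Ball hits and awards a score when destroyed.
; The construction script randomly gives it one or two lives, setting its material and score value to match.
; Each ball hit removes a life, switching to the one-life material or, at zero, calling the CubeDead dispatcher with the score and destroying the actor.
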(event `self.ReceiveBeginPlay`)

(event `self.ReceiveHit`
  (params (MyComp :type "PrimitiveComponent Object Reference") (Other :type "Actor Object Reference") (OtherComp :type "PrimitiveComponent Object Reference") (bSelfMoved :type Boolean) (HitLocation :type "Vector Structure") (HitNormal :type "Vector Structure") (NormalImpulse :type "Vector Structure") (Hit :type "HitResult Structure (by ref)"))
  (cast `/Game/MyGame/Blueprints/BP_Ball` Other)
  (`self.BallIsHit`))

(event `BallIsHit`
  ;[1 0.08854 0.08854] Уничтожение куба с рандомным количеством жизней
  (bind _result (`/Engine/EditorBlueprintResources/StandardMacros.DecrementInt` (`self.Lives`))
    (:`  `
      (if (== _result 1)
        (`PrimitiveComponent.SetMaterial` (`self.Cube`) 0 "/Engine/MapTemplates/Materials/BasicAsset02.BasicAsset02")
        (elif (<= _result 0)
          (`self.CubeDead` (`self.Score`))
          (`self.K2_DestroyActor`))))))

(fn `UserConstructionScript`
  (bind _cube (`self.Cube`))
  ;[0.3066 0.3561 1] Рандомизация количества жизней
  (bind _output_get (set `self.Lives` (`KismetMathLibrary.RandomIntegerInRange` 1 2)))
  ;[1 0.4821 0.4522] Установка материала в зависимости от количества жизней
  (switch `int` _output_get
    (:`1`
      (`PrimitiveComponent.SetMaterial` _cube 0 "/Engine/MapTemplates/Materials/BasicAsset02.BasicAsset02")
      (set `self.Score` 100))
    (:`2`
      (`PrimitiveComponent.SetMaterial` _cube 0 "/Engine/MapTemplates/Materials/BasicAsset01.BasicAsset01")
      (set `self.Score` 250))))