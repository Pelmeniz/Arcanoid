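; BP_CubesGenerator is an actor that spawns a grid of cubes and announces when all of them have died.
; The construction script previews the grid with static mesh components, which BeginPlay destroys before spawning BP_Cube_Child actors at matching offsets.
; Each cube's death event passes score to BP_MyPawn and increments a counter.
; When that counter reaches the spawned cube count, it calls the AllCubesDied dispatcher.
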(event `self.ReceiveBeginPlay`
  (bind (_returnvalue_x _returnvalue_y _returnvalue_z) (`KismetMathLibrary.BreakVector` (`self.K2_GetActorLocation`)))
  (`|ExecutionSequence`
    (:`then_0`
      (bind _returnvalue (`GameplayStatics.GetActorOfClass` "/Game/MyGame/Blueprints/Core/BP_MyPawn.BP_MyPawn_C"))
      (set `self.MyPawn` _returnvalue))
    (:`then_1`
      (for _array_element (`self.PreviewArray`)
        (`ActorComponent.K2_DestroyComponent` _array_element))
      ;[0.1808 0.1829 1] Генерация кубов
      (for _index (range (+ (`self.X`) 1))
        (for _index_2 (range (+ (`self.Y`) 1))
          (bind _returnvalue_2 (`|SpawnActorFromClass` "/Game/MyGame/Blueprints/BP_Cube_Child.BP_Cube_Child_C" (`KismetMathLibrary.MakeTransform` (`KismetMathLibrary.MakeVector` (+ (`KismetMathLibrary.Conv_IntToDouble` (* _index (`self.Padding`))) _returnvalue_x) (+ _returnvalue_y (`KismetMathLibrary.Conv_IntToDouble` (* _index_2 (`self.Padding`)))) _returnvalue_z)) "Undefined" "MultiplyWithRoot" null null))
          (`KismetArrayLibrary.Array_Add` (`self.CubesArray`) _returnvalue_2)))
      (bind _amountcubes (`self.GetCubesForWin`))
      (set `self.AmountCubesForWin` _amountcubes)
      (for _array_element_2 (`self.CubesArray`)
        (add `/Game/MyGame/Blueprints/BP_Cube_Parent.CubeDead` _array_element_2 (delegate `DeathCube`))))))

(event `DeathCube`
  (params (Score :type Integer))
  (`/Game/MyGame/Blueprints/Core/BP_MyPawn.AddedScore` (`self.MyPawn`) Score)
  (`/Engine/EditorBlueprintResources/StandardMacros.IncrementInt` (`self.DeadCubes`)
    (:`  `
      (if (>= (`self.DeadCubes`) (`self.AmountCubesForWin`))
        (`self.AllCubesDied`)))))

(fn `GetCubesForWin`
  (returns (AmountCubes :type Integer))
  (return (`KismetArrayLibrary.Array_Length` (`self.CubesArray`))))

(fn `UserConstructionScript`
  ;[0.1808 0.1829 1] Генерация кубов
  (for _index (range (+ (`self.X`) 1))
    (for _index_2 (range (+ (`self.Y`) 1))
      (bind _returnvalue (`AddComponent|NODE_AddStaticMeshComponent-0` :`RelativeTransform` (`KismetMathLibrary.MakeTransform` (`KismetMathLibrary.MakeVector` (`KismetMathLibrary.Conv_IntToDouble` (* _index (`self.Padding`))) (`KismetMathLibrary.Conv_IntToDouble` (* _index_2 (`self.Padding`)))))))
      (`KismetArrayLibrary.Array_Add` (`self.PreviewArray`) _returnvalue))))